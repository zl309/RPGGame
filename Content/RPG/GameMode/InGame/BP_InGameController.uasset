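; BP_InGameController is the in-game player controller for the RPG, handling cursor setup and camera zoom input.
; On BeginPlay it caches the controlled pawn as BP_MyCharacter, then sets Game and UI input mode with the mouse always locked and the cursor visible.
; Mouse wheel up and down call ZoomIn on that character with opposite-signed fixed steps, leaving the zoom logic to the character.
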(event EventBeginPlay
  (bind _asbp_my_character (Utilities|Casting|CastToBP_MyCharacter (Pawn|GetControlledPawn)))
  (Variables|Default|SetMyCharacter _asbp_my_character)
  (Input|SetInputModeGameandUI self 0 "LockAlways" true false)
  (Variables|Default|SetbShowMouseCursor true))

(event Input|MouseEvents|MouseWheelUp
  (params (Key :type Key%20Structure))
  (:Pressed
    (Default|Zoomin (Variables|Default|GetMyCharacter) -5e+01)))

(event Input|MouseEvents|MouseWheelDown
  (params (Key :type Key%20Structure))
  (:Pressed
    (Default|Zoomin (Variables|Default|GetMyCharacter) 5e+01)))

(fn ConstructionScript)