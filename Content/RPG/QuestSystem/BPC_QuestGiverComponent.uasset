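; Quest giver component that lets its owning actor offer a single data-table quest when interacted with.
; InteractWith asks the player character's quest log component whether the quest is active, then returns the owner's display name.
; If inactive, DisplayQuest looks up the row and opens a W_QuestGiver widget with the quest's details and ID.
; If already active, it only prints a placeholder greeting.
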(event EventBeginPlay)

(event EventTick
  (params (DeltaSeconds :type Float%20%28single-precision%29)))

(fn DisplayQuest
  (bind _questdata (Variables|Default|GetQuestData))
  (bind _returnvalue (Utilities|GetDataTableRow (.datatable _questdata) (.rowname _questdata))
    (:then
      (bind _returnvalue_2 (UserInterface|CreateWidget "/Game/RPG/QuestSystem/UI/W_QuestGiver.W_QuestGiver_C" 0 _returnvalue (.rowname _questdata)))
      (UserInterface|Viewport|AddtoViewport _returnvalue_2 0))))

(fn Interactwith
  (bind _returnvalue (Components|GetOwner))
  (bind _returnvalue_2 (Utilities|GetDisplayName _returnvalue))
  (if (not (Default|QueryActiveQues (Variables|/Game/RPG/DamageSystem/BP_Player.BP_Player_C|GetBPC_QuestLogComponent (CallFunction|GetMyPlayerCharacter)) (.rowname (Variables|Default|GetQuestData))))
    (CallFunction|DisplayQuest)
    (return _returnvalue_2)
    (else
      (Development|PrintString "Hello")
      (return _returnvalue_2))))