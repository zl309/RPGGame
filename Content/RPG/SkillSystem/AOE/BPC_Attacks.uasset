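; BPC_Attacks is a component that spawns area-of-effect skill actors for a lightning strike and a heal.
; LightingStrike passes target, delay, radius and the owning pawn as instigator to BP_Ability_AoE_Lighting.
; Heal line-traces from a valid target toward the ground, spawns BP_Ability_AoE_Heal at the hit and triggers it.
; Both bind the spawned actor's overlap event, but the damage and heal handlers apply no effect yet.
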(event Custom|LightingStrike
  (params (AttackTarget :type Actor%20Object%20Reference) (DelaybeforeStrike :type Float%20%28single-precision%29))
  (bind _returnvalue (Components|GetOwner))
  (bind (_as폰 _bsuccess) (Utilities|Casting|CastToPawn _returnvalue))
  (bind _returnvalue_2 (Game|SpawnActorfromClass "/Game/RPG/SkillSystem/AOE/BP_Ability_AoE_Lighting.BP_Ability_AoE_Lighting_C" (Math|Transform|MakeTransform "0, 0, 0" "0, 0, 0" "1.000000,1.000000,1.000000") "Undefined" 0 DelaybeforeStrike AttackTarget 1e+02 false 0 (select _bsuccess _as폰 0)))
  (EventDispatchers|AssignOnOverlapActor _returnvalue_2 (delegate Custom|DamageEnemyAOE)))

(event Custom|DamageEnemyAOE
  (params (Actor :type Actor%20Object%20Reference)))

(event Custom|Heal
  (params (HealTarget :type Actor%20Object%20Reference))
  (bind _returnvalue (Transformation|GetActorLocation HealTarget))
  (Utilities|IsValid HealTarget
    (:Is%20Valid
      (bind (_outhit _returnvalue_2) (Collision|LineTraceByChannel _returnvalue (* _returnvalue "1.000000,1.000000,-1000.000000") "TraceTypeQuery1" false (Utilities|Array|MakeArray HealTarget) "None"))
      (if _returnvalue_2
        (bind _returnvalue_3 (Game|SpawnActorfromClass "/Game/RPG/SkillSystem/AOE/BP_Ability_AoE_Heal.BP_Ability_AoE_Heal_C" (Math|Transform|MakeTransform (.Location (Collision|BreakHitResult _outhit)) "0, 0, 0" "1.000000,1.000000,1.000000") "Undefined" 0 1.0 5.0 1.2e+02 false 0 0))
        (EventDispatchers|AssignOnOverlapActor _returnvalue_3 (delegate Custom|OnHealTarget))
        (Default|Trigger _returnvalue_3)))))

(event Custom|OnHealTarget
  (params (Actor :type Actor%20Object%20Reference))
  (if (== Actor (stale Custom|Heal HealTarget))
    _))

(event EventBeginPlay)

(event EventTick
  (params (DeltaSeconds :type Float%20%28single-precision%29)))