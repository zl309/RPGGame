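; BP_Ability_AoE is a skill-system actor that performs a one-shot spherical area-of-effect check at its location.
; Trigger, called directly or automatically shortly after BeginPlay when TriggerOnBeginPlay is set, runs a Pawn-only sphere overlap, optionally ignoring the instigator.
; Each hit actor is broadcast through OnOverlapActor and printed by name, leaving effects to listeners.
; The debug sphere draws when DebugSphere is false, inverting the flag's apparent meaning.
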(event Custom|SpawnAOESphere
  (if (Variables|Default|GetDebugSphere)
    _
    (else
      (Rendering|Debug|DrawDebugSphere (Transformation|GetActorLocation) (Variables|Default|GetRadius) 12 "(R=0.000000,G=1.000000,B=0.005394,A=1.000000)" 1.0 1.0)))
  (bind _outactors (Collision|SphereOverlapActors (Transformation|GetActorLocation) (Variables|Default|GetRadius) (Utilities|Array|MakeArray "ObjectTypeQuery3") 0 (select (Variables|Default|GetIgnoreInstigator) (Utilities|Array|MakeArray (Game|GetInstigator)) 0)))
  (for _array_element _outactors
    (Default|CallOnOverlapActor _array_element)
    (Development|PrintString (Utilities|GetDisplayName _array_element))))

(event Custom|Trigger
  (CallFunction|SpawnAOESphere))

(event EventBeginPlay
  (|CallParentFunction)
  (if (Variables|Default|GetTriggerOnBeginPlay)
    (Utilities|FlowControl|Delay 0.2)
    (CallFunction|Trigger)))

(event Collision|EventActorBeginOverlap
  (params (OtherActor :type Actor%20Object%20Reference))
  (|CallParentFunction OtherActor) ; 지금 이 노드는 비활성 상태입니다. \n핀을 끌어서 다른 노드를 연결하면 활성화됩니다.
)

(event EventTick
  (params (DeltaSeconds :type Float%20%28single-precision%29))
  (|CallParentFunction DeltaSeconds) ; 지금 이 노드는 비활성 상태입니다. \n핀을 끌어서 다른 노드를 연결하면 활성화됩니다.
)

(fn ConstructionScript
  (|CallParentFunction))