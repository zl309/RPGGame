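; Base Blueprint for area-of-effect blast abilities in the skill system, adding blast visuals, sound and self-cleanup to the parent's trigger behavior.
; On Trigger, it runs the parent logic, spawns the BlastEffect emitter attached to AbilityRoot and plays BlastSound at the actor's location.
; The actor destroys itself when the particle system finishes, or after a brief delay if no effect is assigned.
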(event Custom|SpawnBlastEffect
  ;[1 1 1] BlastEffect
  (bind _blasteffect (Variables|Default|GetBlastEffect)
    (:then
      (bind _returnvalue (Effects|SpawnEmitterAttached _blasteffect (Variables|Default|GetAbilityRoot) "None"))
      (EventDispatchers|AssignOnSystemFinished _returnvalue (delegate Custom|SystemFinished)))
    (:else
      (Utilities|FlowControl|Delay 0.2)
      (Actor|DestroyActor))))

(event Custom|SystemFinished
  (params (PSystem :type Particle%20System%20Component%20Object%20Reference))
  ;[1 1 1] BlastEffect
  (Actor|DestroyActor))

(event Custom|PlayBlastSound
  ;[1 1 1] BlastSound
  (Audio|PlaySoundatLocation (Variables|Default|GetBlastSound) (Transformation|GetActorLocation) "0, 0, 0" 1.0 1.0 0.0 0 0 0 0))

(event EventBeginPlay
  (|CallParentFunction) ; 지금 이 노드는 비활성 상태입니다. \n핀을 끌어서 다른 노드를 연결하면 활성화됩니다.
)

(event Collision|EventActorBeginOverlap
  (params (OtherActor :type Actor%20Object%20Reference))
  (|CallParentFunction OtherActor) ; 지금 이 노드는 비활성 상태입니다. \n핀을 끌어서 다른 노드를 연결하면 활성화됩니다.
)

(event EventTick
  (params (DeltaSeconds :type Float%20%28single-precision%29))
  (|CallParentFunction DeltaSeconds) ; 지금 이 노드는 비활성 상태입니다. \n핀을 끌어서 다른 노드를 연결하면 활성화됩니다.
)

(event EventTrigger
  ;[1 1 1] 호출
  (|CallParentFunction)
  (CallFunction|SpawnBlastEffect)
  (CallFunction|PlayBlastSound))

(fn ConstructionScript
  (|CallParentFunction))