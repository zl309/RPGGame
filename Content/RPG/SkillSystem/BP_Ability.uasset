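; BP_Ability is an RPG skill actor that starts casting as soon as it spawns.
; It gets the main character widget from the HUD, then either shows a cast bar with a success binding or, without cast time, calls DisplaySkill immediately.
; DisplaySkill fires the CastSuccess dispatcher, while InterruptCasting destroys the actor and fires CastInterrupted.
; ActivateEffect is only a debug-print placeholder.
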(event EventBeginPlay
  (bind _asbp_in_game_hud (Utilities|Casting|CastToBP_InGameHud (HUD|GetHUD (Game|GetPlayerController 0))))
  (Variables|Default|SetHUD%20Widget (Variables|/Game/RPG/GameMode/InGame/BP_InGameHud.BP_InGameHud_C|GetMainCharacterWidget _asbp_in_game_hud))
  (CallFunction|BeginCasting))

(fn ConstructionScript)

(fn BeginCasting
  (if (> (.casttime (Variables|Default|GetAbilityDetails)) 0.0)
    (bind _castbarwidget (Default|DisplayCastBar (Variables|Default|GetHUD%20Widget) self))
    (EventDispatchers|BindEventtoCastSuccessful _castbarwidget (EventDispatchers|CreateEvent :!event DisplaySkill))
    (else
      (CallFunction|DisplaySkill))))

(fn DisplaySkill
  (Development|PrintString "GotoSkillBarWidget1")
  (Default|CallCastSuccess))

(fn InterruptCasting
  (Actor|DestroyActor)
  (Default|CallCastInterrupted))

(fn ActivateEffect
  (Development|PrintString "ActivateEffect"))